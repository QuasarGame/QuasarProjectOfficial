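; Spline mesh actor that builds a deformed static mesh segment between each pair of neighboring spline points in its construction script.
; Each segment takes its position and tangents from the spline, plus a shared roll, collision setting and optional material override on slot 0.
; A per-point Scale transform array drives start and end scale, with its locations repositioned just above each spline point.
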(fn ConstructionScript
  (CallFunction|SetUpSplineMeshes))

(fn MakeSplineMeshComponent
  (params (Transform :type Transform))
  (bind _returnvalue (AddComponent|AddSplineMeshComponent false Transform)) ; X Forward Axis
  (SplineMesh|SetForwardAxis _returnvalue (Utilities|Select :Index (Variables|Default|GetAxis) :Option%200 "X" :Option%201 "X" :Option%202 "X") true)
  (return _returnvalue))

(fn GetLocationsandTangentsforSplinePoint
  (params (Spline%20Component :type Spline%20Component%20Object%20Reference) (Index :type Integer))
  (bind (_location _tangent) (Spline|GetLocationandTangentatSplinePoint Spline%20Component Index "Local"))
  (bind _returnvalue (+ Index 1))
  (bind (_location_2 _tangent_2) (Spline|GetLocationandTangentatSplinePoint Spline%20Component _returnvalue "Local"))
  (return _location _tangent _location_2 _tangent_2))

(fn SetScaleArrayLocations
  (params (Index :type Integer))
  (Utilities|Array|SetArrayElem (Variables|Default|GetScale) Index (Math|Transform|MakeTransform (+ (.Location (Spline|GetLocationandTangentatSplinePoint (Variables|Default|GetSpline1) Index "Local")) "0, 0,50.000000") "0, 0, 0" (.Scale (Math|Transform|BreakTransform (Utilities|Array|Get(acopy) (Variables|Default|GetScale) Index)))) true))

(fn SetUpSplineMeshes
  (bind _scale (Variables|Default|GetScale))
  (bind _roll (Variables|Default|GetRoll))
  (for _index (range 0 (- (Spline|GetNumberOfSplinePoints (Variables|Default|GetSpline1)) 1))
    (bind _output_get (LocalVariables|SetCurrent%20Index _index))
    (CallFunction|SetScaleArrayLocations _output_get)
    (|IsNotLastIndex)
    (Utilities|FlowControl|Sequence
      (:then_0
        ;[1 1 1] Create Component and set mesh
        (bind _splinemesh_component (CallFunction|MakeSplineMeshComponent (|emptytransform)))
        (bind _output_get_2 (LocalVariables|SetCurrentSplineMeshComponent _splinemesh_component))
        (Components|StaticMesh|SetStaticMesh _output_get_2 (Variables|Default|GetMesh))
        (Utilities|Array|Add (Variables|Default|GetSplineMeshComponents) _splinemesh_component))
      (:then_1
        ;[1 1 1] Set Materials
        (CallFunction|SetMaterials (LocalVariables|GetCurrentSplineMeshComponent)))
      (:then_2
        ;[1 1 1] Set Positions and tangents
        (SplineMesh|SetStartandEnd (LocalVariables|GetCurrentSplineMeshComponent) (.Start%20Pos (CallFunction|GetLocationsandTangentsforSplinePoint (Variables|Default|GetSpline1) (LocalVariables|GetCurrent%20Index))) (.Start%20Tangent (CallFunction|GetLocationsandTangentsforSplinePoint (Variables|Default|GetSpline1) (LocalVariables|GetCurrent%20Index))) (.End%20Pos (CallFunction|GetLocationsandTangentsforSplinePoint (Variables|Default|GetSpline1) (LocalVariables|GetCurrent%20Index))) (.End%20Tangent (CallFunction|GetLocationsandTangentsforSplinePoint (Variables|Default|GetSpline1) (LocalVariables|GetCurrent%20Index))) true :!class /Script/Engine.SplineMeshComponent))
      (:then_3
        ;[1 1 1] Set Roll. Todo: Make this controllable per segment
        (Class|SplineMeshComponent|SetStartRoll (LocalVariables|GetCurrentSplineMeshComponent) _roll true)
        (Class|SplineMeshComponent|SetEndRoll (LocalVariables|GetCurrentSplineMeshComponent) _roll true))
      (:then_4
        ;[1 1 1] Set Scale
        (SplineMesh|SetStartScale (LocalVariables|GetCurrentSplineMeshComponent) (Math|Vector2D|MakeVector2D (Math|Float|Max(Float) (.X (Math|Vector|BreakVector (.Scale (Math|Transform|BreakTransform (Utilities|Array|Get(acopy) _scale (LocalVariables|GetCurrent%20Index)))))) (.Y (Math|Vector|BreakVector (.Scale (Math|Transform|BreakTransform (Utilities|Array|Get(acopy) _scale (LocalVariables|GetCurrent%20Index))))))) (.Z (Math|Vector|BreakVector (.Scale (Math|Transform|BreakTransform (Utilities|Array|Get(acopy) _scale (LocalVariables|GetCurrent%20Index))))))) true :!class /Script/Engine.SplineMeshComponent)
        (SplineMesh|SetEndScale (LocalVariables|GetCurrentSplineMeshComponent) (Math|Vector2D|MakeVector2D (Math|Float|Max(Float) (.X (Math|Vector|BreakVector (.Scale (Math|Transform|BreakTransform (Utilities|Array|Get(acopy) _scale (+ (LocalVariables|GetCurrent%20Index) 1)))))) (.Y (Math|Vector|BreakVector (.Scale (Math|Transform|BreakTransform (Utilities|Array|Get(acopy) _scale (+ (LocalVariables|GetCurrent%20Index) 1))))))) (.Z (Math|Vector|BreakVector (.Scale (Math|Transform|BreakTransform (Utilities|Array|Get(acopy) _scale (+ (LocalVariables|GetCurrent%20Index) 1))))))) true :!class /Script/Engine.SplineMeshComponent))
      (:then_5
        ;[1 1 1] set collision
        (Collision|SetCollisionEnabled (LocalVariables|GetCurrentSplineMeshComponent) (Variables|Default|GetCollision)))))
  (return))

(fn SetMaterials
  (params (Spline%20Mesh%20Component :type Spline%20Mesh%20Component%20Object%20Reference))
  (if (> (Utilities|Array|Length (Variables|Default|GetMaterial%20Overwrite)) 0)
    (for _array_element (Variables|Default|GetMaterial%20Overwrite)
      (Utilities|IsValid _array_element
        (:Is%20Valid
          (Rendering|Material|SetMaterial Spline%20Mesh%20Component 0 _array_element)))))
  (return))