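; Warning light actor with two point lights and two spot lights that share one configurable color.
; On BeginPlay it applies LightColor to all four lights, with IntensityPoint driving the point lights and Intensity driving the spot lights.
; The construction script is empty, so these values are applied only once play begins.
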(event EventBeginPlay
  (bind _pointlight1 (Variables|Default|GetPointLight1))
  (bind _pointlight (Variables|Default|GetPointLight))
  (bind _spotlight1 (Variables|Default|GetSpotLight1))
  (bind _spotlight (Variables|Default|GetSpotLight))
  (bind _intensity_point (Variables|Default|GetIntensity_point))
  (bind _intensity (Variables|Default|GetIntensity))
  (bind _lightcolor (Variables|Default|GetLightColor))
  (Rendering|Components|Light|SetLightColor _pointlight1 _lightcolor true)
  (Rendering|Components|Light|SetLightColor _pointlight _lightcolor true)
  (Rendering|Components|Light|SetIntensity _pointlight1 _intensity_point)
  (Rendering|Components|Light|SetIntensity _pointlight _intensity_point)
  (Rendering|Components|Light|SetLightColor _spotlight1 _lightcolor true)
  (Rendering|Components|Light|SetLightColor _spotlight _lightcolor true)
  (Rendering|Components|Light|SetIntensity _spotlight1 _intensity)
  (Rendering|Components|Light|SetIntensity _spotlight _intensity))

(fn ConstructionScript)